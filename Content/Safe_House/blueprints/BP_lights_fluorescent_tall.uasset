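; Tall fluorescent light fixture with configurable hanging chains and a rect light, built entirely in the construction script.
; Stacks static mesh segments at fixed spacing on both sides up to ChainHeight, then optionally adds a rotated end holder on top.
; Chain1 visibility follows StartHolder, but only when EndHolder is enabled.
; LightColor drives both the mesh emissive and RectLight1, whose intensity, radius, indirect and volumetric strength, and mobility are also exposed.
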(fn `UserConstructionScript`
  (bind _light_color (`self.Light Color`))
  (`|ExecutionSequence`
    (:`then_0`
      (for _index (range (+ (`self.Chain Height`) 1))
        (bind _returnvalue (* _index 19.6))
        (`AddComponent|NODE_AddStaticMeshComponent-0` :`RelativeTransform` (`KismetMathLibrary.MakeTransform` (`KismetMathLibrary.MakeVector` 0.0 -70.0 _returnvalue)))
        (`AddComponent|NODE_AddStaticMeshComponent-2` :`RelativeTransform` (`KismetMathLibrary.MakeTransform` (`KismetMathLibrary.MakeVector` 0.0 69.0 _returnvalue))))
      (if (`self.End Holder`)
        (bind _returnvalue_2 (`AddComponent|NODE_AddStaticMeshComponent-1` :`RelativeTransform` (`KismetMathLibrary.MakeTransform` (`KismetMathLibrary.MakeVector` 0.0 0.0 (+ (* _index 19.6) 3.5)))))
        (`SceneComponent.K2_AddRelativeRotation` _returnvalue_2 (struct :`Pitch` 180.0 :`Yaw` 90.0) false false)
        (`SceneComponent.SetVisibility` (`self.Chain1`) (`self.Start Holder`) false)))
    (:`then_1`
      (`MeshComponent.SetVectorParameterValueOnMaterials` (`self.SM_lights_fluorescent_tall`) "Emissive Color" (`KismetMathLibrary.Conv_LinearColorToVector` _light_color))
      (`LightComponent.SetLightColor` (`self.RectLight1`) _light_color true)
      (`LightComponent.SetIntensity` (`self.RectLight1`) (`self.Rect Intensity`))
      (`LocalLightComponent.SetAttenuationRadius` (`self.RectLight1`) (`self.Rect Radius`))
      (`LightComponent.SetIndirectLightingIntensity` (`self.RectLight1`) (`self.Rect Indirect Intensity`))
      (`SceneComponent.SetMobility` (`self.RectLight1`) (`self.Light Mobility`))
      (`LightComponent.SetVolumetricScatteringIntensity` (`self.RectLight1`) (`self.Volumetric Scattering Intensity `)))))