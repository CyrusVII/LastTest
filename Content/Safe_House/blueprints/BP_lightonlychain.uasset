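; Safe House prop Blueprint that procedurally builds a pair of parallel vertical chains, apparently for hanging a light, with no active gameplay logic.
; The construction script stacks two static mesh columns at fixed spacing, repeating up to ChainHeight.
; If EndHolder is set, it adds a rotated mesh centered at the last index.
; StartHolder drives Chain1's visibility, but only within that EndHolder branch.
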(fn `UserConstructionScript`
  (`|ExecutionSequence`
    (:`then_0`
      (for _index (range (+ (`self.Chain Height`) 1))
        (bind _returnvalue (* _index 19.6))
        (`AddComponent|NODE_AddStaticMeshComponent-0` :`RelativeTransform` (`KismetMathLibrary.MakeTransform` (`KismetMathLibrary.MakeVector` 0.0 -70.0 _returnvalue)))
        (`AddComponent|NODE_AddStaticMeshComponent-2` :`RelativeTransform` (`KismetMathLibrary.MakeTransform` (`KismetMathLibrary.MakeVector` 0.0 69.0 _returnvalue))))
      (if (`self.End Holder`)
        (bind _returnvalue_2 (`AddComponent|NODE_AddStaticMeshComponent-1` :`RelativeTransform` (`KismetMathLibrary.MakeTransform` (`KismetMathLibrary.MakeVector` 0.0 0.0 (+ (* _index 19.6) 3.5)))))
        (`SceneComponent.K2_AddRelativeRotation` _returnvalue_2 (struct :`Pitch` 180.0 :`Yaw` 90.0) false false)
        (`SceneComponent.SetVisibility` (`self.Chain1`) (`self.Start Holder`) false)))))