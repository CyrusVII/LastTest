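; BP_decalWall is a wall actor, named as a decal wall, whose collision can be switched on or off.
; On BeginPlay, it reads the CollisionYesNo boolean and sets the SMNWall component to query and physics collision or to no collision.
; Overlap and Tick events are disabled, and the construction script only calls its parent, so the setting applies only at play start.
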(event `self.ReceiveBeginPlay`
  (bind _sm_nwall (`self.SM_NWall`))
  (`parent.ReceiveBeginPlay`)
  (if (`self.CollisionYesNo?`)
    (`PrimitiveComponent.SetCollisionEnabled` _sm_nwall "QueryAndPhysics")
    (else
      (`PrimitiveComponent.SetCollisionEnabled` _sm_nwall "NoCollision"))))

(fn `UserConstructionScript`
  (`parent.UserConstructionScript`))