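; BP_GridDoor is a door Blueprint that swings open or closed depending on a tag check.
; A self-repeating Tick event, started on BeginPlay, calls CheckForTag every half second through a Delay loop.
; The result plays or reverses a timeline, whose track is remapped to the relative yaw of DoorRotation for a quarter-turn swing.
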(event `self.ReceiveBeginPlay`
  (`parent.ReceiveBeginPlay`)
  (`self.Tick`))

(event `Tick`
  (`|ExecutionSequence`
    (:`then_0`
      (bind _all_true (`self.CheckForTag`))
      (if _all_true
        (bind (_direction _newtrack_0) (`Timeline|Timeline` :!label _label)
          (:`Update`
            (`SceneComponent.K2_SetRelativeRotation` (`self.Door_Rotation`) (`KismetMathLibrary.MakeRotator` 0.0 0.0 (`KismetMathLibrary.MapRangeClamped` _newtrack_0 0.0 1.0 0.0 -90.0)) false false)))
        (else
          (goto _label :!via `Reverse`))))
    (:`then_1`
      (`KismetSystemLibrary.Delay` 0.5)
      (`self.Tick`))))

(fn `UserConstructionScript`
  (`parent.UserConstructionScript`))