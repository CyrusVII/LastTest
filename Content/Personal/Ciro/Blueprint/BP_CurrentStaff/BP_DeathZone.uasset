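; BP_DeathZone is a hazard volume that sends a death message to the player and intercepts physics cubes.
; A half-second loop hides it and disables its collision when the count of active tagged BP_Master_Template actors equals Locks.
; When a cube's sphere overlaps and its ButtonRef is valid, it disables the cube's collision and physics, forces a drop if grabbing, then calls TooltipAction on that button.
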(event `self.ReceiveBeginPlay`
  (bind _asgi_last_test (cast `/Game/Personal/Blueprint_Mattia/GI_LastTest` (`GameplayStatics.GetGameInstance`)))
  (set `self.As GI Last Test` _asgi_last_test)
  (`self.Tick`))

(event `Tick`
  (`|ExecutionSequence`
    (:`then_0`
      (bind _returnvalue (`self.CeackForTag`))
      (if _returnvalue
        (`self.SetActorHiddenInGame` true)
        (`PrimitiveComponent.SetCollisionEnabled` (`self.Box`) "NoCollision")
        (else
          (`self.SetActorHiddenInGame` false)
          (`PrimitiveComponent.SetCollisionEnabled` (`self.Box`) "QueryOnly"))))
    (:`then_1`
      (`KismetSystemLibrary.Delay` 0.5)
      (`self.Tick`))))

(event `self.Box.OnComponentBeginOverlap`
  (params (OverlappedComponent :type "PrimitiveComponent Object Reference") (OtherActor :type "Actor Object Reference") (OtherComp :type "PrimitiveComponent Object Reference") (OtherBodyIndex :type Integer) (bFromSweep :type Boolean) (SweepResult :type "HitResult Structure (by ref)"))
  (bind _as_bp_physic_cube (`self.As BP Physic Cube`))
  (bind _staticmesh (`/Game/Personal/Blueprint_Mattia/BP_Switches/BP_Master_Template.StaticMesh` _as_bp_physic_cube))
  (set `self.Other Actor` OtherActor)
  (`|ExecutionSequence`
    (:`then_0`
      (if (== (`self.Other Actor`) (`GameplayStatics.GetPlayerCharacter` 0))
        (message `/Game/Personal/Blueprint_Mattia/BPI_Character.Dead` (`self.Other Actor`))))
    (:`then_1`
      (bind _asbp_physic_cube (cast `/Game/Personal/Blueprint_Mattia/BP_Switches/BP_PhysicCube` OtherActor))
      (if (== (`/Game/Personal/Blueprint_Mattia/BP_Switches/BP_PhysicCube.Sphere` _asbp_physic_cube) OtherComp)
        (bind _output_get (set `self.As BP Physic Cube` _asbp_physic_cube))
        (`/Game/Personal/Blueprint_Mattia/BP_Switches/BP_PhysicCube.Button Ref` _output_get
          (:`then`
            (`PrimitiveComponent.SetCollisionEnabled` (`/Game/Personal/Blueprint_Mattia/BP_Switches/BP_PhysicCube.Box` _as_bp_physic_cube) "NoCollision")
            (`PrimitiveComponent.SetEnableGravity` _staticmesh false)
            (`PrimitiveComponent.SetSimulatePhysics` _staticmesh false)
            (if (`/Game/Personal/Blueprint_Mattia/GI_LastTest.IsGrabbinObject` (`self.As GI Last Test`))
              (message `/Game/Personal/Blueprint_Mattia/BPI_Character.DropGrabbedOject` (`GameplayStatics.GetPlayerCharacter` 0)))
            (`/Game/Personal/Blueprint_Mattia/BP_Switches/BP_Master_Template.Tooltip Action` (`/Game/Personal/Blueprint_Mattia/BP_Switches/BP_PhysicCube.Button Ref` (`self.As BP Physic Cube`))))
          (:`else`))))))

(fn `CeackForTag`
  (returns (ReturnValue :type Boolean))
  (locals (`Locks Open` :type Integer))
  (bind _outactors (`GameplayStatics.GetAllActorsWithTag` (`self.Tag`)))
  (for _array_element _outactors
    (bind _asbp_master_template (cast `/Game/Personal/Blueprint_Mattia/BP_Switches/BP_Master_Template` _array_element))
    (if (`/Game/Personal/Blueprint_Mattia/BP_Switches/BP_Master_Template.Active` _asbp_master_template)
      (`/Engine/EditorBlueprintResources/StandardMacros.IncrementInt` (`local.Locks Open`))))
  (return (== (`local.Locks Open`) (`self.Locks`))))

(fn `UserConstructionScript`
  (locals (LocksOpen :type Integer)))