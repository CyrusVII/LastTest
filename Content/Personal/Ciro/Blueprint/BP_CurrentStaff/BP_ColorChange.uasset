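; Color-change platform that recolors a BP_PhysicCube of a different color to its own PlatformColor.
; On overlap, it makes the player drop the cube, disables physics and pulls it to the platform's Cube position with a Timeline lerp.
; Delays chained off the Timeline update sequence a color-matched Niagara spiral, dissolve-out, value change, respawn and physics restore before the DoOnce resets.
; The construction script tints the platform meshes from PlatformColor.
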(event `self.ReceiveBeginPlay`
  (bind _asbp_first_person_character (cast `/Game/Personal/Blueprint_Mattia/BP_FirstPersonCharacter` (`GameplayStatics.GetPlayerCharacter` 0)))
  (set `self.As BP First Person Character` _asbp_first_person_character))

(event `self.Collision.OnComponentBeginOverlap`
  (params (OverlappedComponent :type "PrimitiveComponent Object Reference") (OtherActor :type "Actor Object Reference") (OtherComp :type "PrimitiveComponent Object Reference") (OtherBodyIndex :type Integer) (bFromSweep :type Boolean) (SweepResult :type "HitResult Structure (by ref)"))
  (bind _as_bp_physic_cube (`self.As BP Physic Cube`))
  (bind _staticmesh (`/Game/Personal/Blueprint_Mattia/BP_Switches/BP_Master_Template.StaticMesh` (`self.As BP Physic Cube`)))
  (bind _asbp_physic_cube (cast `/Game/Personal/Blueprint_Mattia/BP_Switches/BP_PhysicCube` OtherActor))
  (bind _output_get (set `self.As BP Physic Cube` _asbp_physic_cube))
  (if (and (`PrimitiveComponent.IsOverlappingComponent` (`/Game/Personal/Blueprint_Mattia/BP_Switches/BP_PhysicCube.Box` _output_get) (`self.Collision`)) (`|EnumInequality` (`self.PlatformColor`) (`/Game/Personal/Blueprint_Mattia/BP_Switches/BP_PhysicCube.ValueCube` (`self.As BP Physic Cube`))))
    (`/Engine/EditorBlueprintResources/StandardMacros.DoOnce` false :!label _label
      (:`Completed`
        (`/Game/Personal/Blueprint_Mattia/BP_Switches/BP_Master_Template.OlograpichYesNo` (`self.As BP Physic Cube`))
        (set `self.Active` true)
        (set `self.Cube World Location` (`SceneComponent.K2_GetComponentLocation` _staticmesh))
        (`PrimitiveComponent.SetSimulatePhysics` _staticmesh false)
        (`/Game/Personal/Blueprint_Mattia/BP_FirstPersonCharacter.DropObject` (`self.As BP First Person Character`))
        (bind (_direction _newtrack_0) (`Timeline|Timeline` :!via `PlayFromStart`)
          (:`Update`
            (if (`self.Active`)
              (`SceneComponent.K2_SetWorldLocation` (`/Game/Personal/Blueprint_Mattia/BP_Switches/BP_Master_Template.StaticMesh` (`self.As BP Physic Cube`)) (`KismetMathLibrary.VLerp` (`self.Cube World Location`) (`SceneComponent.K2_GetComponentLocation` (`self.Cube`)) _newtrack_0) false false)
              (`KismetSystemLibrary.Delay` 0.3)
              (`self.SetSpiralColor`)
              (`KismetSystemLibrary.Delay` 1.0)
              (`/Game/Personal/Blueprint_Mattia/BP_Switches/BP_PhysicCube.DissolvDestroy` _as_bp_physic_cube)
              (`KismetSystemLibrary.Delay` 1.0)
              (bind _output_get_2 (set `/Game/Personal/Blueprint_Mattia/BP_Switches/BP_PhysicCube.ValueCube` (`self.PlatformColor`) _as_bp_physic_cube))
              (`/Game/Personal/Blueprint_Mattia/BP_Switches/BP_PhysicCube.Constraction Value` _as_bp_physic_cube _output_get_2)
              (`/Game/Personal/Blueprint_Mattia/BP_Switches/BP_PhysicCube.DissolvSpawn` _as_bp_physic_cube)
              (`KismetSystemLibrary.Delay` 1.3)
              (`PrimitiveComponent.SetSimulatePhysics` (`/Game/Personal/Blueprint_Mattia/BP_Switches/BP_Master_Template.StaticMesh` _as_bp_physic_cube) true)
              (`KismetSystemLibrary.Delay` 0.7)
              (`NiagaraComponent.SetAsset` (`self.NS_Spiral`) null false)
              (goto _label :!via `Reset`))))))))

(fn `ColorValue`
  (params (Index :type "/Game/Personal/Blueprint_Mattia/Enum/E_ColorValue Enum" :default "NewEnumerator0"))
  (`MeshComponent.SetVectorParameterValueOnMaterials` (`|MakeArray` (`self.Platform`) (`self.arc4`) (`self.arc3`) (`self.arc2`) (`self.arc6`) (`self.arc1Base`) (`self.arc5`) :!type "MeshComponent Object Reference") "BaseColor" (select `/Game/Personal/Blueprint_Mattia/Enum/E_ColorValue` Index :`NewEnumerator0` (0.0 0.001754 0.572917) :`NewEnumerator1` (0.71875 0.0 0.0) :`NewEnumerator2` (0.84375 0.617612 0.0) :`NewEnumerator3` (1.0 1.0 1.0) :`NewEnumerator5` (0.067708 0.067708 0.067708) :!type "Vector Structure")))

(fn `SetSpiralColor`
  (bind _ns_spiral (`self.NS_Spiral`))
  (switch `/Game/Personal/Blueprint_Mattia/Enum/E_ColorValue` (`self.PlatformColor`)
    (:`NewEnumerator0`
      (`NiagaraComponent.SetAsset` _ns_spiral "/Game/Personal/Ciro/Niagara/NiagaraSpiral/NS_SpiralBlue.NS_SpiralBlue" true))
    (:`NewEnumerator1`
      (`NiagaraComponent.SetAsset` _ns_spiral "/Game/Personal/Ciro/Niagara/NiagaraSpiral/NS_SpiralRed.NS_SpiralRed" true))
    (:`NewEnumerator2`
      (`NiagaraComponent.SetAsset` _ns_spiral "/Game/Personal/Ciro/Niagara/NiagaraSpiral/NS_SpiralYellow.NS_SpiralYellow" true))
    (:`NewEnumerator3`
      (`NiagaraComponent.SetAsset` _ns_spiral "/Game/Personal/Ciro/Niagara/NiagaraSpiral/NS_Spiral.NS_Spiral" true))))

(fn `UserConstructionScript`
  (`self.ColorValue` (`self.PlatformColor`)))