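; BP_ChipLife is a floating chip actor that shows a tooltip on the first-person character when the player is within its sphere.
; Tick bobs the mesh vertically with a time-based sine wave.
; BeginPlay caches the player character, and sphere begin and end overlaps toggle its tooltip.
; Disconnected logic would fill one of two HUD life bars and destroy the chip, but never runs; the Hit event is empty.
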(event `self.ReceiveTick`
  (params (DeltaSeconds :type "Float (single-precision)"))
  (`SceneComponent.K2_SetRelativeLocation` (`self.SM_ChipBase`) (`KismetMathLibrary.MakeVector` 0.0 0.0 (`KismetMathLibrary.MapRangeClamped` (`KismetMathLibrary.Sin` (* (`GameplayStatics.GetTimeSeconds`) 1.0)) -1.0 1.0 0.0 50.0)) false false))

(event `self.Sphere.OnComponentBeginOverlap`
  (params (OverlappedComponent :type "PrimitiveComponent Object Reference") (OtherActor :type "Actor Object Reference") (OtherComp :type "PrimitiveComponent Object Reference") (OtherBodyIndex :type Integer) (bFromSweep :type Boolean) (SweepResult :type "HitResult Structure (by ref)"))
  (bind _as_bp_first_person_character (`self.As BP First Person Character`))
  (if (`PrimitiveComponent.IsOverlappingComponent` (`Character.CapsuleComponent` _as_bp_first_person_character) (`self.Sphere`))
    (`/Game/Personal/Blueprint_Mattia/BP_FirstPersonCharacter.Tooltip` _as_bp_first_person_character true)))

(event `self.Sphere.OnComponentEndOverlap`
  (params (OverlappedComponent :type "PrimitiveComponent Object Reference") (OtherActor :type "Actor Object Reference") (OtherComp :type "PrimitiveComponent Object Reference") (OtherBodyIndex :type Integer))
  (`/Game/Personal/Blueprint_Mattia/BP_FirstPersonCharacter.Tooltip` (`self.As BP First Person Character`) false))

(event `self.ReceiveBeginPlay`
  (bind _asbp_first_person_character (cast `/Game/Personal/Blueprint_Mattia/BP_FirstPersonCharacter` (`GameplayStatics.GetPlayerCharacter` 0)))
  (set `self.As BP First Person Character` _asbp_first_person_character))

(event `Hit`)

(fn `UserConstructionScript`)