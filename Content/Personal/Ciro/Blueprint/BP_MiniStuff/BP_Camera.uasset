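; BP_Camera is a prop that continuously turns its Arrow component to face the player character, apparently as a tracking camera.
; On BeginPlay it caches the Arrow's world location and a reference to the first-person character, which is not used afterward.
; Each Tick it sets the Arrow's world rotation with FindLookAtRotation from that cached start position to the player's current location, without interpolation or limits.
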(event `self.ReceiveBeginPlay`
  (set `self.StartPosition` (`SceneComponent.K2_GetComponentLocation` (`self.Arrow`)))
  (bind _asbp_first_person_character (cast `/Game/Personal/Blueprint_Mattia/BP_FirstPersonCharacter` (`GameplayStatics.GetPlayerCharacter` 0)))
  (set `self.As BP First Person Character_0` _asbp_first_person_character))

(event `self.ReceiveTick`
  (params (DeltaSeconds :type "Float (single-precision)"))
  (`SceneComponent.K2_SetWorldRotation` (`self.Arrow`) (`KismetMathLibrary.FindLookAtRotation` (`self.StartPosition`) (`self.K2_GetActorLocation` (`GameplayStatics.GetPlayerCharacter` 0))) false false))

(fn `UserConstructionScript`)