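; BP_PressColor is an actor with four rect lights and four static meshes, mostly fluorescent fixtures, that can be set to blue, red or yellow.
; The construction script switches on the SetColor variable, setting each light's color and swapping each mesh's first material to the matching light material instance.
; The event graph holds only disabled stub events, so the Blueprint has no runtime logic of its own.
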(fn `UserConstructionScript`
  (bind _array (`|MakeArray` (`self.RectLight`) (`self.RectLight4`) (`self.RectLight5`) (`self.RectLight3`)))
  (bind _array_2 (`|MakeArray` (`self.SM_lights_fluorescent_single4`) (`self.SM_lights_fluorescent_single5`) (`self.StaticMesh`) (`self.SM_lights_fluorescent_single3`)))
  (switch `/Game/Personal/Blueprint_Mattia/Enum/E_ColorValue` (`self.SetColor`)
    (:`NewEnumerator0`
      (`LightComponent.SetLightColor` _array (struct :`R` 0.004391 :`B` 1.0 :`A` 1.0) true)
      (`PrimitiveComponent.SetMaterial` _array_2 0 "/Game/Safe_House/material_instances/MI_light_Blue.MI_light_Blue"))
    (:`NewEnumerator1`
      (`LightComponent.SetLightColor` _array (struct :`R` 1.0 :`A` 1.0) true)
      (`PrimitiveComponent.SetMaterial` _array_2 0 "/Game/Safe_House/material_instances/MI_light_Red.MI_light_Red"))
    (:`NewEnumerator2`
      (`LightComponent.SetLightColor` _array (struct :`R` 1.0 :`G` 0.760525 :`A` 1.0) true)
      (`PrimitiveComponent.SetMaterial` _array_2 0 "/Game/Safe_House/material_instances/MI_light_Yellow.MI_light_Yellow"))))