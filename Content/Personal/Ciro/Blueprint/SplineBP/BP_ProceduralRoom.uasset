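; BP_ProceduralRoom is an actor that configures a PCG graph for a square procedural room or multi-floor building.
; Its construction script derives floor offset and scale, four wall offsets and a pivot correction from wall size, floor size and wall thickness.
; The floor count sets building height, roof offset and a single-floor flag, and the negated actor location becomes the floor-copy offset.
; All values are written as PCG graph instance parameters.
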(event EventBeginPlay)

(event Collision|EventActorBeginOverlap
  (params (OtherActor :type Actor%20Object%20Reference)))

(event EventTick
  (params (DeltaSeconds :type Float%20%28single-precision%29)))

(fn ConstructionScript
  (bind _pcg (Variables|Default|GetPCG))
  (bind _wallsize (Variables|Default|GetWallSize))
  (bind _wallsize_2 (Variables|Default|GetWallSize))
  (bind _wallsize_3 (Variables|Default|GetWallSize))
  (bind _returnvalue (/ _wallsize 2.0))
  (bind _returnvalue_2 (/ _wallsize_3 2.0))
  (bind _returnvalue_3 (/ _wallsize_2 2.0))
  (bind _graphinstance (Variables|/Script/PCG.PCGComponent|GetGraphInstance _pcg))
  ;[0.04916 1 0] Calcolo Pedana Non Centrale
  (Effects|Components|ParticleSystem|SetVectorParameter _graphinstance "FloorOffset" (Math|Vector|MakeVector (* _returnvalue -1.0) _returnvalue 0.0))
  (Effects|Components|ParticleSystem|SetVectorParameter _graphinstance "FloorScale" (Math|Conversions|ToVector(Float) (/ (Variables|Default|GetWallSize) (Variables|Default|GetFloorSize))))
  ;[0.03253 0 1] Calcolo per posizionare i muri
  (Effects|Components|ParticleSystem|SetVectorParameter _graphinstance "WallOffset1" (Math|Vector|MakeVector _returnvalue_2 0.0 0.0))
  (Effects|Components|ParticleSystem|SetVectorParameter _graphinstance "WallOffset2" (Math|Vector|MakeVector (* _returnvalue_2 -1.0) 0.0 0.0))
  (Effects|Components|ParticleSystem|SetVectorParameter _graphinstance "WallOffset3" (Math|Vector|MakeVector 0.0 _returnvalue_3 0.0))
  (Effects|Components|ParticleSystem|SetVectorParameter _graphinstance "WallOffset4" (Math|Vector|MakeVector 0.0 (* _returnvalue_3 -1.0) 0.0))
  (Effects|Components|ParticleSystem|SetVectorParameter _graphinstance "WallOffsetPivot" (Math|Vector|MakeVector (* (/ (Variables|Default|GetWallSize) 2.0) -1.0) (Variables|Default|GetWallThickness) 0.0))
  ;[1 0 0.7929] Floor
  (Effects|Components|ParticleSystem|SetVectorParameter _graphinstance "BuildingHige" (Math|Vector|MakeVector 0.0 0.0 (* 4.8e+02 (- (Variables|Default|GetFloor) 1))))
  (Effects|Components|ParticleSystem|SetVectorParameter _graphinstance "FloorCopyOffset" (* (Transformation|GetActorLocation) -1.0))
  (Effects|Components|ParticleSystem|SetBoolParameter _graphinstance "SingleFloor" (== (Variables|Default|GetFloor) 1))
  (Effects|Components|ParticleSystem|SetVectorParameter _graphinstance "RoofOffset" (Math|Vector|MakeVector 0.0 0.0 (Math|Conversions|ToFloat(Integer) (* (Variables|Default|GetFloor) 475)))))