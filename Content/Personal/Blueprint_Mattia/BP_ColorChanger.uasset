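; BP_ColorChanger is a trigger actor that changes the color value of any BP_PhysicCube entering its capsule.
; On begin overlap, it confirms the cube's Box overlaps the capsule, copies ValueChanger into ValueCube, then calls the cube's ConstractionValue and ColorSwap.
; The construction script sets the changer's own Cube material from ValueChanger (blue, red, yellow or white), with blue using MT_Default.
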(event `self.Capsule.OnComponentBeginOverlap`
  (params (OverlappedComponent :type "PrimitiveComponent Object Reference") (OtherActor :type "Actor Object Reference") (OtherComp :type "PrimitiveComponent Object Reference") (OtherBodyIndex :type Integer) (bFromSweep :type Boolean) (SweepResult :type "HitResult Structure (by ref)"))
  (bind _asbp_physic_cube (cast `/Game/Personal/Blueprint_Mattia/BP_Switches/BP_PhysicCube` OtherActor))
  (if (`PrimitiveComponent.IsOverlappingComponent` (`/Game/Personal/Blueprint_Mattia/BP_Switches/BP_PhysicCube.Box` _asbp_physic_cube) (`self.Capsule`))
    (bind _output_get (set `/Game/Personal/Blueprint_Mattia/BP_Switches/BP_PhysicCube.ValueCube` (`self.ValueChanger`) _asbp_physic_cube))
    (`/Game/Personal/Blueprint_Mattia/BP_Switches/BP_PhysicCube.Constraction Value` _asbp_physic_cube _output_get)
    (`/Game/Personal/Blueprint_Mattia/BP_Switches/BP_PhysicCube.ColorSwap` _asbp_physic_cube)))

(fn `UserConstructionScript`
  (bind _cube (`self.Cube`))
  (switch `/Game/Personal/Blueprint_Mattia/Enum/E_ColorValue` (`self.ValueChanger`)
    (:`NewEnumerator0`
      (`PrimitiveComponent.SetMaterial` _cube 0 "/Game/Personal/Blueprint_Mattia/Material/MT_Default.MT_Default"))
    (:`NewEnumerator1`
      (`PrimitiveComponent.SetMaterial` _cube 0 "/Game/Personal/Blueprint_Mattia/Mesh/Material/MI_Red.MI_Red"))
    (:`NewEnumerator2`
      (`PrimitiveComponent.SetMaterial` _cube 0 "/Game/Personal/Blueprint_Mattia/Mesh/Material/MI_Yellow.MI_Yellow"))
    (:`NewEnumerator3`
      (`PrimitiveComponent.SetMaterial` _cube 0 "/Game/Personal/Blueprint_Mattia/Material/MI_White.MI_White"))))