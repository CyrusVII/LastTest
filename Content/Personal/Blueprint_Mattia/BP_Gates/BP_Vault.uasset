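; Vault gate that opens and closes in response to the inherited OnLocksOpened event.
; When locks open, timelines spin the handle and slide the locker bolt, then swing the door after a one-second delay.
; When locks close, separate reverse timelines swing the door back, then re-engage the bolt and handle, gated by a DoOnce that each opening resets.
; The construction script applies StartRotation to the door.
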(event `self.ReceiveBeginPlay`
  (`self.CheckForTag` self)
  (add `self.OnLocksOpened` (delegate `OnLocksOpened_Event`)))

(event `OnLocksOpened_Event` :!signature `self.OnLocksOpened`
  (params (Result :type Boolean))
  (if Result
    (`|ExecutionSequence`
      (:`then_0`
        (bind (_direction _newtrack_0) (`Timeline|Timeline_0`)
          (:`Update`
            (`|ExecutionSequence`
              (:`then_0`
                (`SceneComponent.K2_SetRelativeRotation` (`self.Handle`) (`KismetMathLibrary.MakeRotator` 0.0 (`KismetMathLibrary.MapRangeClamped` _newtrack_0 0.0 1.0 0.0 360.0)) false false))
              (:`then_1`
                (`SceneComponent.K2_SetRelativeLocation` (`self.locker`) (`KismetMathLibrary.MakeVector` (`KismetMathLibrary.MapRangeClamped` _newtrack_0 0.0 1.0 353.712611 61.669183) 790.381618 -0.42949) false false))))
          (:`Finished`
            (`KismetSystemLibrary.Delay` 1.0)
            (bind (_direction_2 _newtrack_0_2) (`Timeline|Timeline`)
              (:`Update`
                (`SceneComponent.K2_SetRelativeRotation` (`self.Door_Rotation`) (`KismetMathLibrary.MakeRotator` 0.0 0.0 (`KismetMathLibrary.MapRangeClamped` _newtrack_0_2 0.0 1.0 (`self.Out Range A`) (`self.Out Range B`))) false false))))))
      (:`then_1`
        (goto _label :!via `Reset`)))
    (else
      (`/Engine/EditorBlueprintResources/StandardMacros.DoOnce` true :!label _label
        (:`Completed`
          (bind (_direction_3 _newtrack_0_3) (`Timeline|Timeline_1` :!via `ReverseFromEnd`)
            (:`Update`
              (`SceneComponent.K2_SetRelativeRotation` (`self.Door_Rotation`) (`KismetMathLibrary.MakeRotator` 0.0 0.0 (`KismetMathLibrary.MapRangeClamped` _newtrack_0_3 0.0 1.0 (`self.Out Range A`) (`self.Out Range B`))) false false))
            (:`Finished`
              (`KismetSystemLibrary.Delay` 1.0)
              (bind (_direction_4 _newtrack_0_4) (`Timeline|Timeline_2` :!via `ReverseFromEnd`)
                (:`Update`
                  (`|ExecutionSequence`
                    (:`then_0`
                      (`SceneComponent.K2_SetRelativeRotation` (`self.Handle`) (`KismetMathLibrary.MakeRotator` 0.0 (`KismetMathLibrary.MapRangeClamped` _newtrack_0_4 0.0 1.0 0.0 360.0)) false false))
                    (:`then_1`
                      (`SceneComponent.K2_SetRelativeLocation` (`self.locker`) (`KismetMathLibrary.MakeVector` (`KismetMathLibrary.MapRangeClamped` _newtrack_0_4 0.0 1.0 353.712611 61.669183) 790.381618 -0.42949) false false))))))))))))

(fn `UserConstructionScript`
  (`parent.UserConstructionScript`)
  (`SceneComponent.K2_SetRelativeRotation` (`self.Door_Rotation`) (`KismetMathLibrary.MakeRotator` 0.0 0.0 (`self.Start Rotation`)) false false))