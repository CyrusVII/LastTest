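; Iron window gate that slides vertically toward MoveZ while its CheckForTag test passes, and reverses otherwise.
; A self-repeating custom Tick event, started at BeginPlay, polls the tag every half second to play or reverse a Timeline.
; Timeline updates remap its value into root Z, feeding current world coordinates into the relative location.
; The construction script swaps in a shutter mesh when Bars is set.
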(event `self.ReceiveBeginPlay`
  (`self.Tick`))

(event `Tick`
  (bind (_returnvalue_x _returnvalue_y) (`KismetMathLibrary.BreakVector` (`SceneComponent.K2_GetComponentLocation` (`self.DefaultSceneRoot`))))
  (bind (_returnvalue_x_2 _returnvalue_y_2 _returnvalue_z) (`KismetMathLibrary.BreakVector` (`SceneComponent.K2_GetComponentLocation` (`self.DefaultSceneRoot`))))
  (`|ExecutionSequence`
    (:`then_0`
      (bind _all_true (`self.CheckForTag`))
      (if _all_true
        (bind (_direction _moving) (`Timeline|Timeline` :!label _label)
          (:`Update`
            (`SceneComponent.K2_SetRelativeLocation` (`self.DefaultSceneRoot`) (`KismetMathLibrary.MakeVector` _returnvalue_x _returnvalue_y (`KismetMathLibrary.MapRangeClamped` _moving 0.0 25.0 _returnvalue_z (`self.MoveZ`))) false false)))
        (else
          (goto _label :!via `Reverse`))))
    (:`then_1`
      (`KismetSystemLibrary.Delay` 0.5)
      (`self.Tick`))))

(fn `UserConstructionScript`
  (if (`self.Bars`)
    (`StaticMeshComponent.SetStaticMesh` (`self.StaticMesh`) "/Game/Safe_House/meshes/SM_windows_shutter_03.SM_windows_shutter_03")))