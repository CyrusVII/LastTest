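; Sliding gate door Blueprint with left and right meshes, apparently derived from a parent gate class.
; Tick calls CheckForTag, then calls Tick again after a short Delay; BeginPlay is empty.
; A Timeline that slides both panels apart along X, or reverses to close them, is left disconnected, so this graph does not move the door itself.
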(event `self.ReceiveBeginPlay`)

(event `Tick`
  (`|ExecutionSequence`
    (:`then_0`
      (`self.CheckForTag` null))
    (:`then_1`
      (`KismetSystemLibrary.Delay` 0.5)
      (`self.Tick`))))

(fn `UserConstructionScript`
  (`parent.UserConstructionScript`))