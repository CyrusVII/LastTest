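; BP_Gate_Template is a template gate that works out whether its linked switches have unlocked it.
; CheckForTag gathers BPI_Switches actors carrying TagToCheck and passes each a gate reference through the interface.
; CheckForOpening polls those switches for access, increments LocksOpen without resetting it, and fires OnLocksOpened with whether the count equals Locks.
; The gate's visible opening response is not implemented here.
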(fn `CheckForOpening`
  (locals (LocksOpen :type Integer))
  (bind _returnvalue (== (`local.LocksOpen`) (`self.Locks`)))
  (for _array_element (`self.Out Actors`)
    (bind _active (message `/Game/Personal/Blueprint_Mattia/BP_Switches/BPI_Switches.GetAccess` _array_element))
    (if _active
      (`/Engine/EditorBlueprintResources/StandardMacros.IncrementInt` (`local.LocksOpen`))))
  (if _returnvalue
    _
    (else
      _))
  (`self.OnLocksOpened` _returnvalue))

(fn `CheckForTag`
  (params (`Gate Ref In` :type "/Game/Personal/Blueprint_Mattia/BP_Gates/BP_Gate_Template Object Reference"))
  (locals (LocksOpen :type Integer))
  (bind _out_actors (`self.Out Actors`))
  (bind _outactors (`GameplayStatics.GetAllActorsWithInterface` "/Game/Personal/Blueprint_Mattia/BP_Switches/BPI_Switches.BPI_Switches_C"))
  (for _array_element _outactors
    (if (`self.ActorHasTag` _array_element (`self.Tag to Check`))
      (`KismetArrayLibrary.Array_AddUnique` _out_actors _array_element)
      (message `/Game/Personal/Blueprint_Mattia/BP_Switches/BPI_Switches.GateRef` _out_actors `Gate Ref In`))))

(fn `UserConstructionScript`)