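; BP_DestructionWall is a color-coded puzzle wall that rejects physics cubes of a different color, or every cube when set to Cube Destroyer.
; Its value picks the wall material and switches between StartingValue and NewValue on the OnLocksOpened event, with sound cues.
; When a cube's Sphere overlaps the Box and is rejected, the wall disables its physics, drops any grabbed object and calls TooltipAction on the cube's linked button.
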(event `self.ReceiveBeginPlay`
  (bind _asgi_last_test (cast `/Game/Personal/Blueprint_Mattia/GI_LastTest` (`GameplayStatics.GetGameInstance`)))
  (set `self.As GI Last Test` _asgi_last_test)
  (`self.CheckForTag` self)
  (add `self.OnLocksOpened` (delegate `OnLocksOpened_Event`))
  (`/Engine/EditorBlueprintResources/StandardMacros.DoOnce` false
    (:`Completed`
      (set `self.CubeValue` (`self.StartingValue`)))))

(event `OnLocksOpened_Event` :!signature `self.OnLocksOpened`
  (params (Result :type Boolean))
  (if Result
    (`self.SetWallColor` (`self.NewValue`))
    (`GameplayStatics.PlaySound2D` "/Game/Personal/SOUND_EFFECT/SomethingHappened/SC_WallDisapper.SC_WallDisapper" 1.0 1.0 0.0 null null)
    (goto _label :!via `Reset`)
    (else
      (`self.SetWallColor` (`self.StartingValue`))
      (`/Engine/EditorBlueprintResources/StandardMacros.DoOnce` false :!label _label
        (:`Completed`
          (`GameplayStatics.PlaySound2D` "/Game/Personal/SOUND_EFFECT/SomethingHappened/SC_WallAppear.SC_WallAppear" 1.0 1.0 0.0 null null))))))

(event `self.Box.OnComponentBeginOverlap`
  (params (OverlappedComponent :type "PrimitiveComponent Object Reference") (OtherActor :type "Actor Object Reference") (OtherComp :type "PrimitiveComponent Object Reference") (OtherBodyIndex :type Integer) (bFromSweep :type Boolean) (SweepResult :type "HitResult Structure (by ref)"))
  (bind _staticmesh (`/Game/Personal/Blueprint_Mattia/BP_Switches/BP_Master_Template.StaticMesh` (`self.As BP Physic Cube`)))
  (bind _asbp_physic_cube (cast `/Game/Personal/Blueprint_Mattia/BP_Switches/BP_PhysicCube` OtherActor))
  (if (== OtherComp (`/Game/Personal/Blueprint_Mattia/BP_Switches/BP_PhysicCube.Sphere` _asbp_physic_cube))
    (bind _output_get (set `self.As BP Physic Cube` _asbp_physic_cube))
    (`/Engine/EditorBlueprintResources/StandardMacros.IsValid` _output_get
      (:`Is Valid`
        (if (or (`|EnumEquality` (`self.CubeValue`) "NewEnumerator4") (`|EnumInequality` (`self.CubeValue`) (`/Game/Personal/Blueprint_Mattia/BP_Switches/BP_PhysicCube.ValueCube` (`self.As BP Physic Cube`))))
          (`/Engine/EditorBlueprintResources/StandardMacros.DoOnce` false :!label _label_2
            (:`Completed`
              (`PrimitiveComponent.SetEnableGravity` _staticmesh false)
              (`PrimitiveComponent.SetSimulatePhysics` _staticmesh false)
              (if (`/Game/Personal/Blueprint_Mattia/GI_LastTest.IsGrabbinObject` (`self.As GI Last Test`))
                (message `/Game/Personal/Blueprint_Mattia/Interface/BPI_Character.DropGrabbedOject` (`GameplayStatics.GetPlayerCharacter` 0)))
              (`/Game/Personal/Blueprint_Mattia/BP_Switches/BP_Master_Template.Tooltip Action` (`/Game/Personal/Blueprint_Mattia/BP_Switches/BP_PhysicCube.Button Ref` (`self.As BP Physic Cube`)))
              (goto _label_2 :!via `Reset`))))))))

(fn `SetWallColor`
  (params (Selection :type "/Game/Personal/Blueprint_Mattia/Enum/E_ColorValue Enum" :default "NewEnumerator0"))
  (bind _wall (`self.Wall`))
  (bind _output_get (set `self.CubeValue` Selection))
  (switch `/Game/Personal/Blueprint_Mattia/Enum/E_ColorValue` _output_get
    (:`NewEnumerator0`
      (`PrimitiveComponent.SetMaterial` _wall 0 "/Game/Personal/Blueprint_Mattia/Mesh/Material/MT_WallCube.MT_WallCube"))
    (:`NewEnumerator1`
      (`PrimitiveComponent.SetMaterial` _wall 0 "/Game/Personal/Blueprint_Mattia/Mesh/Material/MI_RedWallCube.MI_RedWallCube"))
    (:`NewEnumerator2`
      (`PrimitiveComponent.SetMaterial` _wall 0 "/Game/Personal/Blueprint_Mattia/Mesh/Material/MI_YellowWallCube.MI_YellowWallCube"))
    (:`NewEnumerator3`
      (`PrimitiveComponent.SetMaterial` _wall 0 "/Game/Personal/Blueprint_Mattia/Mesh/Material/MTI_WallCube_Neutre.MTI_WallCube_Neutre"))
    (:`NewEnumerator4`
      (`PrimitiveComponent.SetMaterial` _wall 0 "/Game/Personal/Blueprint_Mattia/Mesh/Material/MT_NoCube.MT_NoCube"))))

(fn `UserConstructionScript`
  (`self.SetWallColor` (`self.StartingValue`)))