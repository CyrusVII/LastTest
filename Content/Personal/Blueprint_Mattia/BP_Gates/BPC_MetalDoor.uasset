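; Metal door Blueprint that swings on its yaw axis according to the AllTrue condition.
; A self-calling Tick event polls AllTrue every 0.3 seconds, with paired DoOnce gates limiting reactions to state changes.
; A timeline plays or reverses with door sounds, mapping its track to a configurable yaw range.
; The construction script sets the starting yaw, and BeginPlay also calls CheckForTag on itself.
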(event `self.ReceiveBeginPlay`
  (`self.Tick`)
  (`self.CheckForTag` self))

(event `Tick`
  (`|ExecutionSequence`
    (:`then_0`
      (if (`self.AllTrue`)
        (`|ExecutionSequence`
          (:`then_0`
            (`/Engine/EditorBlueprintResources/StandardMacros.DoOnce` false :!label _label
              (:`Completed`
                (`GameplayStatics.PlaySoundAtLocation` "/Game/Personal/SOUND_EFFECT/SC_DoorClose.SC_DoorClose" (0.0 0.0 0.0) (struct) 1.0 1.0 0.0 null null null null)
                (bind (_direction _newtrack_0) (`Timeline|Timeline_0` :!label _label_2)
                  (:`Update`
                    (`SceneComponent.K2_SetRelativeRotation` (`self.Door_Rotation`) (`KismetMathLibrary.MakeRotator` 0.0 0.0 (`KismetMathLibrary.MapRangeClamped` _newtrack_0 0.0 1.0 (`self.OutRangeA`) (`self.OutRangeB`))) false false))))))
          (:`then_1`
            (goto _label_3 :!via `Reset`)))
        (else
          (`|ExecutionSequence`
            (:`then_0`
              (goto _label :!via `Reset`))
            (:`then_1`
              (`/Engine/EditorBlueprintResources/StandardMacros.DoOnce` true :!label _label_3
                (:`Completed`
                  (`GameplayStatics.PlaySoundAtLocation` "/Game/Personal/SOUND_EFFECT/SC_DoorOpen.SC_DoorOpen" (0.0 0.0 0.0) (struct) 1.0 1.0 0.0 null null null null)
                  (goto _label_2 :!via `Reverse`))))))))
    (:`then_1`
      (`KismetSystemLibrary.Delay` 0.3)
      (`self.Tick`))))

(fn `UserConstructionScript`
  (`parent.UserConstructionScript`)
  (`SceneComponent.K2_SetRelativeRotation` (`self.Door_Rotation`) (`KismetMathLibrary.MakeRotator` 0.0 0.0 (`self.SetStartRot atino`)) false false))