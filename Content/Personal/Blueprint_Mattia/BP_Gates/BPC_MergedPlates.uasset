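; Gate-folder child Blueprint, apparently for merged plates, that slides its root along X while a tag check passes.
; A self-calling Tick event polls CheckForTag every half second, playing a Timeline on success and reversing it otherwise.
; The Timeline value is range-mapped from the current world X toward MoveX and written as relative location, with the start re-read on each update.
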(event `self.ReceiveBeginPlay`
  (`parent.ReceiveBeginPlay`)
  (`self.Tick`))

(event `Tick`
  (bind _defaultsceneroot (`self.DefaultSceneRoot`))
  (bind (_returnvalue_x _returnvalue_y _returnvalue_z) (`KismetMathLibrary.BreakVector` (`SceneComponent.K2_GetComponentLocation` _defaultsceneroot)))
  (bind _returnvalue_x_2 (`KismetMathLibrary.BreakVector` (`SceneComponent.K2_GetComponentLocation` (`self.DefaultSceneRoot`))))
  (`|ExecutionSequence`
    (:`then_0`
      (bind _all_true (`self.CheckForTag`))
      (if _all_true
        (bind (_direction _moving) (`Timeline|Timeline` :!label _label)
          (:`Update`
            (`SceneComponent.K2_SetRelativeLocation` _defaultsceneroot (`KismetMathLibrary.MakeVector` (`KismetMathLibrary.MapRangeClamped` _moving 0.0 35.0 _returnvalue_x_2 (`self.MoveX`)) _returnvalue_y _returnvalue_z) false false)))
        (else
          (goto _label :!via `Reverse`))))
    (:`then_1`
      (`KismetSystemLibrary.Delay` 0.5)
      (`self.Tick`))))

(fn `UserConstructionScript`
  (`parent.UserConstructionScript`))