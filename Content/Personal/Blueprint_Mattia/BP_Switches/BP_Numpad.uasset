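; Numpad switch that unlocks a gate when the player enters the correct keypad code.
; On BeginPlay it passes itself to its child-actor number buttons, which can report digits, backspace or confirm through ButtonEntered.
; Digits replace a dotted placeholder and stop at the code's length.
; Confirm shows right/wrong text, sound and LED, then after a delay updates Active and asks the linked gate to recheck, with GetAccess exposing that state.
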(event `self.ReceiveBeginPlay`
  (`TextRenderComponent.K2_SetText` (`self.EnterCodeText`) (`KismetTextLibrary.Conv_StringToText` (`KismetStringLibrary.GetSubstring` "..............." 0 (`KismetStringLibrary.Len` (`self.Keypad Code`)))))
  (bind _output_get (set `self.Buttons Array` (`|MakeArray` (`self.B0`) (`self.B1`) (`self.B2`) (`self.B3`) (`self.B4`) (`self.B5`) (`self.B6`) (`self.B7`) (`self.B8`) (`self.B9`) (`self.BDel`) (`self.BOk`))))
  (for _array_element _output_get
    (bind _asbp_number_button (cast `/Game/Personal/Blueprint_Mattia/BP_Switches/BP_NumberButton` (`ChildActorComponent.ChildActor` _array_element)))
    (set `/Game/Personal/Blueprint_Mattia/BP_Switches/BP_NumberButton.Pad Actor Ref` self _asbp_number_button)))

(event `Button Entered`
  (params (Value :type Text) (`Confirmed?` :type Boolean) (BackSpace :type Boolean))
  (bind _entercodetext (`self.EnterCodeText`))
  (`|ExecutionSequence`
    (:`then_0`
      (if `Confirmed?`
        (`self.Confirm`)
        (elif BackSpace
          (`self.backSpace`)
          (elif (`self.Can Enter`)
            (`TextRenderComponent.K2_SetText` _entercodetext (`KismetTextLibrary.Conv_StringToText` (`KismetStringLibrary.Replace` (`KismetTextLibrary.Conv_TextToString` (`TextRenderComponent.Text` (`self.EnterCodeText`))) (`KismetStringLibrary.GetSubstring` "........." 0 (`KismetStringLibrary.Len` (`self.Keypad Code`))))))
            (`TextRenderComponent.K2_SetText` _entercodetext (`KismetTextLibrary.Conv_StringToText` (`KismetStringLibrary.Concat_StrStr` (`KismetTextLibrary.Conv_TextToString` (`TextRenderComponent.Text` (`self.EnterCodeText`))) (`KismetTextLibrary.Conv_TextToString` Value))))))))
    (:`then_1`
      (if (>= (`KismetStringLibrary.Len` (`KismetTextLibrary.Conv_TextToString` (`TextRenderComponent.Text` (`self.EnterCodeText`)))) (`KismetStringLibrary.Len` (`self.Keypad Code`)))
        (set `self.Can Enter` false)
        (else
          (set `self.Can Enter` true))))))

(event `Backspace`
  (bind _returnvalue (`KismetTextLibrary.Conv_TextToString` (`TextRenderComponent.Text` (`self.EnterCodeText`))))
  (`TextRenderComponent.K2_SetText` (`self.EnterCodeText`) (`KismetTextLibrary.Conv_StringToText` (`KismetStringLibrary.GetSubstring` _returnvalue 0 (- (`KismetStringLibrary.Len` _returnvalue) 1)))))

(event `Confirm`
  (if (`KismetStringLibrary.EqualEqual_StrStr` (`self.Keypad Code`) (`KismetTextLibrary.Conv_TextToString` (`TextRenderComponent.Text` (`self.EnterCodeText`))))
    (set `self.Can Enter` false)
    (`TextRenderComponent.K2_SetText` (`self.EnterCodeText`) (`KismetSystemLibrary.MakeLiteralText` (`self.Code Correct`)))
    (`GameplayStatics.PlaySoundAtLocation` "/Game/Personal/SOUND_EFFECT/ObjectSound/Numpad/SC_CorrectCode.SC_CorrectCode" (0.0 0.0 0.0) (struct) 1.0 1.0 0.0 null null null null)
    (`MeshComponent.SetScalarParameterValueOnMaterials` (`self.Green Led`) "Emissive" 2.0)
    (`KismetSystemLibrary.Delay` 2.0)
    (`TextRenderComponent.K2_SetText` (`self.EnterCodeText`) "")
    (`MeshComponent.SetScalarParameterValueOnMaterials` (`self.Green Led`) "Emissive" 0.0)
    (set `self.Active` true)
    (`/Game/Personal/Blueprint_Mattia/BP_Gates/BP_Gate_Template.CheckForOpening` (`self.Gate Ref In`))
    (else
      (set `self.Can Enter` false)
      (`TextRenderComponent.K2_SetText` (`self.EnterCodeText`) (`KismetSystemLibrary.MakeLiteralText` (`self.Code Wrong`)))
      (`GameplayStatics.PlaySoundAtLocation` "/Game/Personal/SOUND_EFFECT/ObjectSound/Numpad/SC_WrongCode.SC_WrongCode" (0.0 0.0 0.0) (struct) 1.0 1.0 0.0 null null null null)
      (`MeshComponent.SetScalarParameterValueOnMaterials` (`self.Red Led`) "Emissive" 2.0)
      (`KismetSystemLibrary.Delay` 2.0)
      (`TextRenderComponent.K2_SetText` (`self.EnterCodeText`) "")
      (set `self.Can Enter` true)
      (`MeshComponent.SetScalarParameterValueOnMaterials` (`self.Red Led`) "Emissive" 0.0)
      (set `self.Active` false)
      (`/Game/Personal/Blueprint_Mattia/BP_Gates/BP_Gate_Template.CheckForOpening` (`self.Gate Ref In`)))))

(fn `GateRef`
  (params (`Gate Ref In` :type "/Game/Personal/Blueprint_Mattia/BP_Gates/BP_Gate_Template Object Reference"))
  (returns (`Gate Ref Out` :type "/Game/Personal/Blueprint_Mattia/BP_Gates/BP_Gate_Template Object Reference"))
  (bind _output_get (set `self.Gate Ref In` `Gate Ref In`))
  (return _output_get))

(fn `GetAccess`
  (returns (Active :type Boolean))
  (return (`self.Active`)))

(fn `Grab`
  (returns (`Master Grab Ref` :type "/Game/Personal/Blueprint_Mattia/BP_Switches/BP_Master_Template Object Reference"))
  (return null))

(fn `UserConstructionScript`)