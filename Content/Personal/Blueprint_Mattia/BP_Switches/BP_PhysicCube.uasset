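; BP_PhysicCube is a grabbable cube whose color value drives its emissive look, set in the construction script; BeginPlay stores its spawn point and starting value.
; OlograpichYesNo toggles between solid and color-matched hologram materials.
; A dissolve timeline plays forward to destroy and reverse to spawn, allowing grabbing only near zero dissolve.
; While grabbable, TooltipActive briefly shows an outline and widget through a retriggerable delay.
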(event `self.ReceiveBeginPlay`
  (set `self.SpawnPoint` (`self.K2_GetActorLocation`))
  (set `self.StartingValue` (`self.ValueCube`)))

(event `/Game/Personal/Blueprint_Mattia/BP_Switches/BPI_Switches.Tooltip Active`
  (params (`Character Ref` :type "/Game/Personal/Blueprint_Mattia/BP_FirstPersonCharacter Object Reference"))
  (if (`self.CanGrabCube?`)
    (`PrimitiveComponent.SetRenderCustomDepth` (`self.StaticMesh`) true)
    (`SceneComponent.SetVisibility` (`self.Widget`) true false)
    (`KismetSystemLibrary.RetriggerableDelay` 0.12)
    (`PrimitiveComponent.SetRenderCustomDepth` (`self.StaticMesh`) false)
    (`SceneComponent.SetVisibility` (`self.Widget`) false false)))

(event `ColorSwap`
  (bind _staticmesh (`self.StaticMesh`))
  ;[1 1 1] RobaDaPassare
  (switch `/Game/Personal/Blueprint_Mattia/Enum/E_ColorValue` (`self.ValueCube`) :!label _label
    (:`NewEnumerator0`
      (`PrimitiveComponent.SetMaterial` _staticmesh 0 "/Game/Personal/Ciro/Material/MT_Ologram/MI_OlogramBlue.MI_OlogramBlue"))
    (:`NewEnumerator1`
      (`PrimitiveComponent.SetMaterial` _staticmesh 0 "/Game/Personal/Ciro/Material/MT_Ologram/MI_OlogramRed.MI_OlogramRed"))
    (:`NewEnumerator2`
      (`PrimitiveComponent.SetMaterial` _staticmesh 0 "/Game/Personal/Ciro/Material/MT_Ologram/MI_OlogramYellow.MI_OlogramYellow"))
    (:`NewEnumerator3`
      (`PrimitiveComponent.SetMaterial` _staticmesh 0 "/Game/Personal/Ciro/Material/MT_Ologram/MI_OlogramWhite.MI_OlogramWhite"))
    (:`NewEnumerator5`
      (`PrimitiveComponent.SetMaterial` _staticmesh 0 "/Game/Personal/Ciro/Material/MT_Ologram/MI_OlogramNeutre.MI_OlogramNeutre")))
  (set `self.Condition` false))

(event `self.OlograpichYesNo`
  ;[1 1 1] RobaDaPassare
  (if (`self.Condition`)
    (goto _label)
    (else
      (`PrimitiveComponent.SetMaterial` (`self.StaticMesh`) 0 "/Game/Personal/Ciro/Asset/SM_CurrentActor/Cube/SciFi_FloorTile.SciFi_FloorTile")
      (`self.Constraction Value` (`self.ValueCube`))
      (set `self.Condition` true))))

(event `DissolvDestroy`
  ;[1 1 1] RobaDaPassare
  (bind (_direction _newtrack_0) (`Timeline|Timeline` :!via `PlayFromStart` :!label _label_2)
    (:`Update`
      (`MeshComponent.SetScalarParameterValueOnMaterials` (`self.StaticMesh`) "Animation" _newtrack_0)
      (if (<= _newtrack_0 0.05)
        (set `self.CanGrabCube?` true)
        (else
          (set `self.CanGrabCube?` false))))))

(event `DissolvSpawn`
  ;[1 1 1] RobaDaPassare
  (goto _label_2 :!via `ReverseFromEnd`))

(fn `ClearColor`
  (params (NewParam :type "/Game/Personal/Blueprint_Mattia/Enum/E_ColorValue Enum" :default "NewEnumerator0"))
  (`MeshComponent.SetScalarParameterValueOnMaterials` (`self.StaticMesh`) (select `/Game/Personal/Blueprint_Mattia/Enum/E_ColorValue` NewParam :`NewEnumerator0` "BlueEmissive" :`NewEnumerator1` "RedEmissive" :`NewEnumerator2` "YellowEmissive" :`NewEnumerator3` "NeutreEmissive" :!type "Name") 0.0))

(fn `Constraction Value`
  (params (Value :type "/Game/Personal/Blueprint_Mattia/Enum/E_ColorValue Enum" :default "NewEnumerator0"))
  (`self.ClearColor` (`self.ClearScalar`))
  (`MeshComponent.SetScalarParameterValueOnMaterials` (`self.StaticMesh`) (select `/Game/Personal/Blueprint_Mattia/Enum/E_ColorValue` Value :`NewEnumerator0` "BlueEmissive" :`NewEnumerator1` "RedEmissive" :`NewEnumerator2` "YellowEmissive" :`NewEnumerator3` "NeutreEmissive" :!type "Name") 1.0)
  (`MeshComponent.SetVectorParameterValueOnMaterials` (`self.StaticMesh`) "ColorParamater" (select `/Game/Personal/Blueprint_Mattia/Enum/E_ColorValue` (`self.ValueCube`) :`NewEnumerator0` (0.0 0.001754 0.572917) :`NewEnumerator1` (0.71875 0.0 0.0) :`NewEnumerator2` (0.84375 0.617612 0.0) :`NewEnumerator3` (1.0 1.0 1.0) :`NewEnumerator5` (0.067708 0.067708 0.067708) :!type "Vector Structure"))
  (set `self.ClearScalar` Value))

(fn `DisableGrab`
  (`PrimitiveComponent.SetCollisionResponseToChannel` (`self.StaticMesh`) "ECC_GameTraceChannel2" "ECR_Ignore")
  (`WidgetComponent.SetWidget` (`self.Widget`) null))

(fn `UserConstructionScript`
  (`self.Constraction Value` (`self.ValueCube`)))