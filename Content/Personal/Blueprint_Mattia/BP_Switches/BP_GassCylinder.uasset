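; Gas cylinder switch prop that performs a one-time valve-style turn and steam release when its TooltipAction event fires.
; A timeline rotates the static mesh in yaw, then turns off its custom depth rendering.
; A steam emitter then spawns at the SmokeSpawn transform and is destroyed after a short delay.
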(event `/Game/Personal/Blueprint_Mattia/BP_Switches/BPI_Switches.Tooltip Action`
  (bind _staticmesh (`self.StaticMesh`))
  (bind (_returnvalue_location _returnvalue_rotation _returnvalue_scale) (`KismetMathLibrary.BreakTransform` (`SceneComponent.K2_GetComponentToWorld` (`self.SmokeSpawn`))))
  (`/Engine/EditorBlueprintResources/StandardMacros.DoOnce` false
    (:`Completed`
      (bind (_direction _newtrack_0) (`Timeline|Timeline` :!via `PlayFromStart`)
        (:`Update`
          (`SceneComponent.K2_SetRelativeRotation` _staticmesh (`KismetMathLibrary.MakeRotator` 0.0 0.0 (* _newtrack_0 -1.0)) false false))
        (:`Finished`
          (`PrimitiveComponent.SetRenderCustomDepth` _staticmesh false)
          (bind _returnvalue (`GameplayStatics.SpawnEmitterAtLocation` "/Game/Realistic_Starter_VFX_Pack_Vol2/Particles/Smoke/P_Steam_A.P_Steam_A" _returnvalue_location _returnvalue_rotation _returnvalue_scale))
          (`KismetSystemLibrary.Delay` 2.5)
          (`ActorComponent.K2_DestroyComponent` _returnvalue))))))

(fn `UserConstructionScript`)