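; BP_Master_Template is a template Blueprint in the switches folder for objects the first-person character can target and grab.
; TooltipActive shows the character's tooltip, an optional widget and custom-depth rendering, then a short retriggerable delay hides them once calls stop.
; Grab makes the mesh ignore Pawn collision and returns itself, while Release restores blocking.
; GateRef stores a gate reference, GetAccess returns the Active flag, and OlograpichYesNo is an empty event.
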(event `OlograpichYesNo`)

(event `/Game/Personal/Blueprint_Mattia/BP_Switches/BPI_Switches.Tooltip Active`
  (params (`Character Ref` :type "/Game/Personal/Blueprint_Mattia/BP_FirstPersonCharacter Object Reference"))
  (bind _widget (`self.Widget`))
  (set `self.First Person Character` `Character Ref`)
  (`|ExecutionSequence`
    (:`then_0`
      (if (and (not (`SceneComponent.bVisible` _widget)) (`self.Show Widget`))
        (`SceneComponent.SetVisibility` _widget true false)))
    (:`then_1`
      (`/Game/Personal/Blueprint_Mattia/BP_FirstPersonCharacter.Tooltip` `Character Ref` true)
      (bind _staticmesh (`self.StaticMesh`)
        (:`then`
          (`PrimitiveComponent.SetRenderCustomDepth` _staticmesh true))
        (:`else`
          _))
      (`KismetSystemLibrary.RetriggerableDelay` 0.12)
      (`/Game/Personal/Blueprint_Mattia/BP_FirstPersonCharacter.Tooltip` `Character Ref` false)
      (`SceneComponent.SetVisibility` (`self.Widget`) false false)
      (bind _staticmesh_2 (`self.StaticMesh`)
        (:`then`
          (`PrimitiveComponent.SetRenderCustomDepth` _staticmesh_2 false))
        (:`else`)))))

(event `/Game/Personal/Blueprint_Mattia/BP_Switches/BPI_Switches.Release`
  (`PrimitiveComponent.SetCollisionResponseToChannel` (`self.StaticMesh`) "ECC_Pawn" "ECR_Block"))

(fn `GateRef`
  (params (`Gate Ref In` :type "/Game/Personal/Blueprint_Mattia/BP_Gates/BP_Gate_Template Object Reference"))
  (returns (`Gate Ref Out` :type "/Game/Personal/Blueprint_Mattia/BP_Gates/BP_Gate_Template Object Reference"))
  (set `self.Gate Ref ` `Gate Ref In`)
  (return null))

(fn `GetAccess`
  (returns (Active :type Boolean))
  (return (`self.Active`)))

(fn `Grab`
  (returns (`Master Grab Ref` :type "/Game/Personal/Blueprint_Mattia/BP_Switches/BP_Master_Template Object Reference"))
  (`PrimitiveComponent.SetCollisionResponseToChannel` (`self.StaticMesh`) "ECC_Pawn" "ECR_Ignore")
  (return self))

(fn `UserConstructionScript`)