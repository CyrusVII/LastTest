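; BP_NumberButton is one key of a security keypad, with its digit, DEL or OK mesh picked from Number in the construction script.
; TooltipActive shows outline and tooltip, using a retriggerable delay to clear them once calls stop.
; TooltipAction reports the key to PadActorRef, then a timeline presses the mesh, clicks and reverses, with a flag preventing repeats on return.
; GateRef, GetAccess and Grab are stubs.
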(event `/Game/Personal/Blueprint_Mattia/BP_Switches/BPI_Switches.Tooltip Active`
  (params (`Character Ref` :type "/Game/Personal/Blueprint_Mattia/BP_FirstPersonCharacter Object Reference"))
  (bind _staticmesh (`self.StaticMesh`))
  (`PrimitiveComponent.SetRenderCustomDepth` _staticmesh true)
  (`/Game/Personal/Blueprint_Mattia/BP_FirstPersonCharacter.Tooltip` `Character Ref` true)
  (`KismetSystemLibrary.RetriggerableDelay` 0.12)
  (`PrimitiveComponent.SetRenderCustomDepth` _staticmesh false)
  (`/Game/Personal/Blueprint_Mattia/BP_FirstPersonCharacter.Tooltip` `Character Ref` false))

(event `/Game/Personal/Blueprint_Mattia/BP_Switches/BPI_Switches.Tooltip Action`
  (`/Game/Personal/Blueprint_Mattia/BP_Switches/BP_Numpad.Button Entered` (`self.Pad Actor Ref`) (`self.NoText`) (`self.ConfirmedButton?`) (`self.Back Space Button?`))
  (set `self.Sound?` true)
  (bind (_direction _newtrack_0) (`Timeline|Button - Timeline`)
    (:`Update`
      (`SceneComponent.K2_SetRelativeLocation` (`self.StaticMesh`) (`KismetMathLibrary.MakeVector` 0.0 _newtrack_0) false false))
    (:`Finished`
      (if (`self.Sound?`)
        (`GameplayStatics.PlaySoundAtLocation` "/Game/Personal/SOUND_EFFECT/ObjectSound/Numpad/SC_NumberClick.SC_NumberClick" (0.0 0.0 0.0) (struct) 1.0 1.0 0.0 null null null null)
        (`TimelineComponent.Reverse` (`self.Button - Timeline`))
        (set `self.Sound?` false)))))

(fn `GateRef`
  (params (`Gate Ref In` :type "/Game/Personal/Blueprint_Mattia/BP_Gates/BP_Gate_Template Object Reference"))
  (returns (`Gate Ref Out` :type "/Game/Personal/Blueprint_Mattia/BP_Gates/BP_Gate_Template Object Reference"))
  (return null))

(fn `GetAccess`
  (returns (Active :type Boolean))
  (return false))

(fn `Grab`
  (returns (`Master Grab Ref` :type "/Game/Personal/Blueprint_Mattia/BP_Switches/BP_Master_Template Object Reference"))
  (return null))

(fn `UserConstructionScript`
  (`StaticMeshComponent.SetStaticMesh` (`self.StaticMesh`) (select `int` (`self.Number`) :`0` "/Game/Personal/Blueprint_Mattia/Mesh/Textures_Shield/SecurityShield_trama_BTN_00.SecurityShield_trama_BTN_00" :`1` "/Game/Personal/Blueprint_Mattia/Mesh/Textures_Shield/SecurityShield_trama_BTN_01.SecurityShield_trama_BTN_01" :`2` "/Game/Personal/Blueprint_Mattia/Mesh/Textures_Shield/SecurityShield_trama_BTN_02.SecurityShield_trama_BTN_02" :`3` "/Game/Personal/Blueprint_Mattia/Mesh/Textures_Shield/SecurityShield_trama_BTN_03.SecurityShield_trama_BTN_03" :`4` "/Game/Personal/Blueprint_Mattia/Mesh/Textures_Shield/SecurityShield_trama_BTN_04.SecurityShield_trama_BTN_04" :`5` "/Game/Personal/Blueprint_Mattia/Mesh/Textures_Shield/SecurityShield_trama_BTN_05.SecurityShield_trama_BTN_05" :`6` "/Game/Personal/Blueprint_Mattia/Mesh/Textures_Shield/SecurityShield_trama_BTN_06.SecurityShield_trama_BTN_06" :`7` "/Game/Personal/Blueprint_Mattia/Mesh/Textures_Shield/SecurityShield_trama_BTN_07.SecurityShield_trama_BTN_07" :`8` "/Game/Personal/Blueprint_Mattia/Mesh/Textures_Shield/SecurityShield_trama_BTN_08.SecurityShield_trama_BTN_08" :`9` "/Game/Personal/Blueprint_Mattia/Mesh/Textures_Shield/SecurityShield_trama_BTN_09.SecurityShield_trama_BTN_09" :`10` "/Game/Personal/Blueprint_Mattia/Mesh/Textures_Shield/SecurityShield_trama_BTN_DEL.SecurityShield_trama_BTN_DEL" :`11` "/Game/Personal/Blueprint_Mattia/Mesh/Textures_Shield/SecurityShield_trama_BTN_OK.SecurityShield_trama_BTN_OK" :!type "StaticMesh Object Reference")))