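; BP_CubeRespawnButton is an interactable button that resets its linked BP_PhysicCube to its spawn point and starting value.
; On its tooltip action, a timeline animates the press and reverses while the cube releases grab, dissolves and is destroyed.
; A replacement cube then dissolves in and swaps references with the button, keeping the two-way link.
; A DoOnce with delayed reset blocks repeated presses during the sequence.
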(event `self.ReceiveBeginPlay`
  (`parent.ReceiveBeginPlay`)
  (`KismetSystemLibrary.Delay` 1.0)
  (bind _cube_ref (`self.Cube Ref`)
    (:`then`
      (set `/Game/Personal/Blueprint_Mattia/BP_Switches/BP_PhysicCube.Button Ref` self _cube_ref))
    (:`else`)))

(event `/Game/Personal/Blueprint_Mattia/BP_Switches/BPI_Switches.Tooltip Action`
  (`/Engine/EditorBlueprintResources/StandardMacros.DoOnce` false :!label _label
    (:`Completed`
      (`|ExecutionSequence`
        (:`then_0`
          (bind (_direction _newtrack_2) (`Timeline|Button - Timeline`)
            (:`Update`
              (`SceneComponent.K2_SetRelativeLocation` (`self.StaticMesh`) (`KismetMathLibrary.MakeVector` 0.0 _newtrack_2) false false)
              (`KismetSystemLibrary.RetriggerableDelay` 0.1)
              (`TimelineComponent.Reverse` (`self.Button - Timeline`)))))
        (:`then_1`
          (bind _cube_ref (`self.Cube Ref`)
            (:`then`
              (set `self.Spawn Point` (`/Game/Personal/Blueprint_Mattia/BP_Switches/BP_PhysicCube.SpawnPoint` _cube_ref))
              (set `self.Starting Value` (`/Game/Personal/Blueprint_Mattia/BP_Switches/BP_PhysicCube.StartingValue` _cube_ref))
              (`/Game/Personal/Blueprint_Mattia/BP_Switches/BP_PhysicCube.DisableGrab` _cube_ref)
              (`/Game/Personal/Blueprint_Mattia/BP_Switches/BP_PhysicCube.DissolvDestroy` _cube_ref)
              (`KismetSystemLibrary.Delay` 2.0)
              (`self.K2_DestroyActor` _cube_ref)
              (bind _returnvalue (`|SpawnActorFromClass` "/Game/Personal/Blueprint_Mattia/BP_Switches/BP_PhysicCube.BP_PhysicCube_C" (`KismetMathLibrary.MakeTransform` (`self.Spawn Point`)) "Undefined" "MultiplyWithRoot" null (`self.Starting Value`) null))
              (`MeshComponent.SetScalarParameterValueOnMaterials` (`/Game/Personal/Blueprint_Mattia/BP_Switches/BP_Master_Template.StaticMesh` _returnvalue) "Animation" 1.0)
              (`/Game/Personal/Blueprint_Mattia/BP_Switches/BP_PhysicCube.DissolvSpawn` _returnvalue)
              (bind _output_get (set `self.Cube Ref` _returnvalue))
              (set `/Game/Personal/Blueprint_Mattia/BP_Switches/BP_PhysicCube.Button Ref` self _output_get))
            (:`else`)))
        (:`then_2`
          (`KismetSystemLibrary.Delay` 3.5)
          (goto _label :!via `Reset`))))))

(fn `UserConstructionScript`
  (`parent.UserConstructionScript`))