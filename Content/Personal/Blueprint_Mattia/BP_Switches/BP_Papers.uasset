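; BP_Papers is a placeable paper prop, such as a blueprint, map or snapshot, that highlights itself and shows a player tooltip.
; The construction script picks its static mesh from the Paper selection.
; TooltipActive turns on the character's tooltip and the mesh's custom depth, then a short retriggerable delay switches both off once calls stop.
; BeginPlay runs the parent logic and clears ShowWidget.
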(event `self.ReceiveBeginPlay`
  (`parent.ReceiveBeginPlay`)
  (set `self.Show Widget` false))

(event `/Game/Personal/Blueprint_Mattia/BP_Switches/BPI_Switches.Tooltip Active`
  (params (`Character Ref` :type "/Game/Personal/Blueprint_Mattia/BP_FirstPersonCharacter Object Reference"))
  (`/Game/Personal/Blueprint_Mattia/BP_FirstPersonCharacter.Tooltip` (`self.First Person Character`) true)
  (bind _staticmesh (`self.StaticMesh`)
    (:`then`
      (`PrimitiveComponent.SetRenderCustomDepth` _staticmesh true))
    (:`else`
      _))
  (`KismetSystemLibrary.RetriggerableDelay` 0.12)
  (`/Game/Personal/Blueprint_Mattia/BP_FirstPersonCharacter.Tooltip` (`self.First Person Character`) false)
  (bind _staticmesh_2 (`self.StaticMesh`)
    (:`then`
      (`PrimitiveComponent.SetRenderCustomDepth` _staticmesh_2 false))
    (:`else`)))

(fn `UserConstructionScript`
  (`parent.UserConstructionScript`)
  (`StaticMeshComponent.SetStaticMesh` (`self.StaticMesh`) (select `/Game/Personal/Blueprint_Mattia/Enum/E_Papers` (`self.Paper`) :`NewEnumerator0` "/Game/Safe_House/meshes/SM_papers_blueprints_03.SM_papers_blueprints_03" :`NewEnumerator1` "/Game/Safe_House/meshes/SM_papers_map_02.SM_papers_map_02" :`NewEnumerator2` "/Game/Safe_House/meshes/SM_papers_snapshot_02.SM_papers_snapshot_02" :`NewEnumerator3` "/Game/Safe_House/meshes/SM_papers_snapshot_06.SM_papers_snapshot_06" :`NewEnumerator4` "/Game/Safe_House/meshes/SM_papers_snapshot_07.SM_papers_snapshot_07" :!type "StaticMesh Object Reference")))