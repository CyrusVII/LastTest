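; Puzzle pressure plate that activates when a BP_PhysicCube with a matching value overlaps it, then tells its linked gate to check for opening.
; A Timeline rotates four side meshes while pulling the cube to the box, with physics off until it finishes and the player forced to drop it.
; The cube leaving deactivates the plate and, with a valid gate, rechecks it and reverses the animation.
; ConstructionValue colors the lights by pressure value.
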(event `self.ReceiveBeginPlay`
  (`parent.ReceiveBeginPlay`)
  (set `self.Show Widget` false))

(event `self.Box.OnComponentBeginOverlap`
  (params (OverlappedComponent :type "PrimitiveComponent Object Reference") (OtherActor :type "Actor Object Reference") (OtherComp :type "PrimitiveComponent Object Reference") (OtherBodyIndex :type Integer) (bFromSweep :type Boolean) (SweepResult :type "HitResult Structure (by ref)"))
  (bind _staticmesh (`/Game/Personal/Blueprint_Mattia/BP_Switches/BP_Master_Template.StaticMesh` (`self.As BP Physic Cube`)))
  (bind _asbp_physic_cube (cast `/Game/Personal/Blueprint_Mattia/BP_Switches/BP_PhysicCube` OtherActor))
  (set `self.As BP Physic Cube` _asbp_physic_cube)
  (if (and (`PrimitiveComponent.IsOverlappingComponent` (`/Game/Personal/Blueprint_Mattia/BP_Switches/BP_PhysicCube.Box` _asbp_physic_cube) (`self.Box`)) (`|EnumEquality` (`self.ValuePressure`) (`/Game/Personal/Blueprint_Mattia/BP_Switches/BP_PhysicCube.ValueCube` (`self.As BP Physic Cube`))))
    (`/Engine/EditorBlueprintResources/StandardMacros.DoOnce` false :!label _label
      (:`Completed`
        (`self.OlograpichYesNo` (`self.As BP Physic Cube`))
        (set `self.Active` true)
        (bind _gate_ref_ (`self.Gate Ref `)
          (:`then`
            (`/Game/Personal/Blueprint_Mattia/BP_Gates/BP_Gate_Template.CheckForOpening` _gate_ref_))
          (:`else`
            _))
        (set `self.CubeWorldLocation` (`SceneComponent.K2_GetComponentLocation` _staticmesh))
        (`PrimitiveComponent.SetSimulatePhysics` _staticmesh false)
        (message `/Game/Personal/Blueprint_Mattia/BPI_Character.DropObjectCauseOtherForce` (`GameplayStatics.GetPlayerCharacter` 0))
        (bind (_direction _newtrack_0) (`Timeline|Timeline` :!label _label_2)
          (:`Update`
            (`|ExecutionSequence`
              (:`then_0`
                (bind _returnvalue (`KismetMathLibrary.MapRangeClamped` _newtrack_0 0.0 1.0 90.0))
                (`SceneComponent.K2_SetRelativeRotation` (`self.SM_PressureSide1`) (`KismetMathLibrary.MakeRotator` _returnvalue 0.0 -180.0) false false)
                (`SceneComponent.K2_SetRelativeRotation` (`self.SM_PressureSide2`) (`KismetMathLibrary.MakeRotator` 180.0 (`KismetMathLibrary.MapRangeClamped` _newtrack_0 0.0 1.0 90.0 180.0)) false false)
                (`SceneComponent.K2_SetRelativeRotation` (`self.SM_PressureSide3`) (`KismetMathLibrary.MakeRotator` 0.0 _returnvalue) false false)
                (`SceneComponent.K2_SetRelativeRotation` (`self.SM_PressureSide4`) (`KismetMathLibrary.MakeRotator` _returnvalue) false false)
                (`/Engine/EditorBlueprintResources/StandardMacros.DoOnce` false
                  (:`Completed`
                    (if (not (`self.CanBringBackCube?`))
                      (`PrimitiveComponent.SetCollisionResponseToChannel` (`/Game/Personal/Blueprint_Mattia/BP_Switches/BP_Master_Template.StaticMesh` (`self.As BP Physic Cube`)) "ECC_Visibility" "ECR_Ignore")))))
              (:`then_1`
                (if (`self.Active`)
                  (`SceneComponent.K2_SetWorldLocation` (`/Game/Personal/Blueprint_Mattia/BP_Switches/BP_Master_Template.StaticMesh` (`self.As BP Physic Cube`)) (`KismetMathLibrary.VLerp` (`self.CubeWorldLocation`) (`SceneComponent.K2_GetComponentLocation` (`self.Box`)) _newtrack_0) false false)))))
          (:`Finished`
            (bind _as_bp_physic_cube (`self.As BP Physic Cube`)
              (:`then`
                (`PrimitiveComponent.SetSimulatePhysics` (`/Game/Personal/Blueprint_Mattia/BP_Switches/BP_Master_Template.StaticMesh` _as_bp_physic_cube) true)
                (`self.Release` _as_bp_physic_cube))
              (:`else`))))))))

(event `self.Box.OnComponentEndOverlap`
  (params (OverlappedComponent :type "PrimitiveComponent Object Reference") (OtherActor :type "Actor Object Reference") (OtherComp :type "PrimitiveComponent Object Reference") (OtherBodyIndex :type Integer))
  (if (== OtherActor (`self.As BP Physic Cube`))
    (set `self.Active` false)
    (bind _gate_ref_ (`self.Gate Ref `)
      (:`then`
        (`/Game/Personal/Blueprint_Mattia/BP_Gates/BP_Gate_Template.CheckForOpening` _gate_ref_)
        (`|ExecutionSequence`
          (:`then_0`
            (goto _label :!via `Reset`))
          (:`then_1`
            (goto _label_2 :!via `Reverse`))))
      (:`else`))))

(fn `ConstructionValue`
  (`LightComponent.SetLightColor` (`|MakeArray` null null null null :!type "LightComponent Object Reference") (select `/Game/Personal/Blueprint_Mattia/Enum/E_ColorValue` (`self.ValuePressure`) :`NewEnumerator0` (struct :`R` 0.008614 :`B` 0.458333 :`A` 1.0) :`NewEnumerator1` (struct :`R` 0.458333 :`A` 1.0) :`NewEnumerator2` (struct :`R` 1.0 :`G` 0.848436 :`A` 1.0) :!type "LinearColor Structure") true)
  (`PrimitiveComponent.SetMaterial` (`|MakeArray` null null null null :!type "PrimitiveComponent Object Reference") 0 null))

(fn `UserConstructionScript`
  (`parent.UserConstructionScript`))