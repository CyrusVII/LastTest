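; BP_LaserReflect is a laser reflector that bounces an incoming BP_Laser off the point it hits.
; LaserBounce spawns a new laser at the impact point, copying colour and spawn reference, with rotation from mirroring the incoming direction by the surface normal.
; It caches the hit data and destroys the bounced laser when the hit ends or the position check fails, leaving respawning to a later call.
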(fn `Calculate Rotation`
  (params (`Impact Point` :type "Vector Structure") (`Impact Normal` :type "Vector Structure") (`Trace Start` :type "Vector Structure"))
  (returns (ReturnValue :type "Rotator Structure"))
  (return (`KismetMathLibrary.MakeRotFromZ` (`KismetMathLibrary.MirrorVectorByNormal` (- `Impact Point` `Trace Start`) `Impact Normal`))))

(fn `Laser Bounce`
  (params (`Hit?` :type Boolean) (`Laser Ref` :type "/Game/Personal/Blueprint_Mattia/BP_Switches/Lasers/BP_Laser Object Reference") (`Hit Result` :type "HitResult Structure"))
  (returns (`Spawn New Laser?` :type "/Game/Personal/Blueprint_Mattia/BP_Switches/Lasers/BP_Laser Object Reference"))
  (bind _laser_ref (`local.Laser Ref`))
  (bind (_bblockinghit _binitialoverlap _time _distance _location _impactpoint _normal _impactnormal _physmat _hitactor _hitcomponent _hitbonename _bonename _hititem _elementindex _faceindex _tracestart) (`GameplayStatics.BreakHitResult` (`local.Hit Result`)))
  (`self.Bounced laser`
    (:`then`
      (if (and (`KismetMathLibrary.EqualExactly_VectorVector` (`self.Impact Point`) _impactpoint) (`KismetMathLibrary.EqualExactly_VectorVector` (`self.Impact Normal`) _impactnormal) (`KismetMathLibrary.EqualExactly_VectorVector` (`self.Trace Start`) _tracestart))
        (if (not (`local.Hit?`)) :!label _label
          (`self.K2_DestroyActor` (`self.Bounced laser`)))
        (return null)
        (else
          (`self.K2_DestroyActor` (`self.Bounced laser`)))))
    (:`else`
      (set `self.Impact Point` _impactpoint)
      (set `self.Impact Normal` _impactnormal)
      (set `self.Trace Start` _tracestart)
      (bind _returnvalue (`|SpawnActorFromClass` "/Game/Personal/Blueprint_Mattia/BP_Switches/Lasers/BP_Laser.BP_Laser_C" (`KismetMathLibrary.MakeTransform` (`self.Impact Point`) (`self.Calculate Rotation` (`self.Impact Point`) (`self.Impact Normal`) (`self.Trace Start`))) "Undefined" "MultiplyWithRoot" null (`/Game/Personal/Blueprint_Mattia/BP_Switches/Lasers/BP_LaserParent.LaserColor` _laser_ref) (`/Game/Personal/Blueprint_Mattia/BP_Switches/Lasers/BP_LaserParent.SpawnReference` _laser_ref) null))
      (set `self.Bounced laser` _returnvalue)
      (goto _label))))

(fn `UserConstructionScript`
  (`parent.UserConstructionScript`))