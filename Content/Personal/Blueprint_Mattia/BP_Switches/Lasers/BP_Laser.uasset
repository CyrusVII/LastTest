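; Laser beam actor that shoots along its up vector and notifies objects it hits, such as bouncers or receivers implementing BPI_Laser.
; Each tick a thin box trace finds the blocking actor and stretches the beam mesh to the hit distance or full range.
; It sends LaserBounceMessage every frame to a steadily hit actor and a release message when the target changes.
; BeginPlay tints the beam through a dynamic material.
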(event `self.ReceiveBeginPlay`
  (`self.ChangeColor`))

(event `self.ReceiveTick`
  (params (DeltaSeconds :type "Float (single-precision)"))
  (`self.CheckFrontalActor`))

(fn `ChangeColor`
  (bind _returnvalue (`PrimitiveComponent.CreateDynamicMaterialInstance` (`self.SM_Parent`) 0 "/Game/Personal/Blueprint_Mattia/BP_Switches/Lasers/MT_Laser.MT_Laser" "None"))
  (`MaterialInstanceDynamic.SetVectorParameterValue` _returnvalue "Color" (`self.LaserColor`)))

(fn `CheckFrontalActor`
  (locals (`Hit Actor` :type "Actor Object Reference") (LaserRange :type "Float (double-precision)" :default 3000.0))
  (bind _returnvalue (`self.GetActorUpVector`))
  (bind _returnvalue_2 (+ (`self.K2_GetActorLocation`) (* _returnvalue 2.0)))
  (bind _outhit (`KismetSystemLibrary.BoxTraceSingle` _returnvalue_2 (+ _returnvalue_2 (* _returnvalue (`local.LaserRange`))) (0.5 0.5 0.5) (struct) "TraceTypeQuery1"))
  (bind _output_get (set `self.LaserHitResult` _outhit))
  (bind (_bblockinghit _binitialoverlap _time _distance _location _impactpoint _normal _impactnormal _physmat _hitactor) (`GameplayStatics.BreakHitResult` _output_get))
  (set `local.Hit Actor` _hitactor)
  (`SceneComponent.SetWorldScale3D` (`self.SM_Parent`) (`KismetMathLibrary.MakeVector` 0.05 0.05 (`KismetMathLibrary.SelectFloat` (/ (+ _distance 1.0) 100.0) (/ (`local.LaserRange`) 100.0) _bblockinghit)))
  (`|ExecutionSequence`
    (:`then_0`
      (if (!= (`local.Hit Actor`) (`self.Last Hit Actor`))
        (if (`KismetSystemLibrary.DoesImplementInterface` (`self.Last Hit Actor`) "/Game/Personal/Blueprint_Mattia/BP_Switches/Lasers/BPI_Laser.BPI_Laser_C")
          (message `/Game/Personal/Blueprint_Mattia/BP_Switches/Lasers/BPI_Laser.Laser Bounce` (`self.Last Hit Actor`) false self (`self.LaserHitResult`)))
        (elif (`KismetSystemLibrary.DoesImplementInterface` (`local.Hit Actor`) "/Game/Personal/Blueprint_Mattia/BP_Switches/Lasers/BPI_Laser.BPI_Laser_C")
          (message `/Game/Personal/Blueprint_Mattia/BP_Switches/Lasers/BPI_Laser.Laser Bounce` (`local.Hit Actor`) true self (`self.LaserHitResult`)))))
    (:`then_1`
      (set `self.Last Hit Actor` (`local.Hit Actor`)))))

(fn `UserConstructionScript`
  (`parent.UserConstructionScript`))