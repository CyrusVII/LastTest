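; BP_LaserCube is a puzzle cube that redirects an incoming laser along its arrow direction.
; LaserBounce spawns an attached BP_Laser at the Arrow, copying the source laser's color and spawn reference, and destroys it when the hit ends.
; It also binds to the source laser's destruction, with OnDead removing the spawned beam.
; TooltipActive shows a custom-depth highlight and widget, using a short retriggerable delay to hide them once calls stop.
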(event `OnDead`
  (params (DestroyedActor :type "Actor Object Reference"))
  (`self.K2_DestroyActor` (`self.LaserSpawn`)))

(event `/Game/Personal/Blueprint_Mattia/BP_Switches/BPI_Switches.Tooltip Active`
  (params (`Character Ref` :type "/Game/Personal/Blueprint_Mattia/BP_FirstPersonCharacter Object Reference"))
  (`PrimitiveComponent.SetRenderCustomDepth` (`self.StaticMesh`) true)
  (`SceneComponent.SetVisibility` (`self.Widget`) true false)
  (`KismetSystemLibrary.RetriggerableDelay` 0.12)
  (`PrimitiveComponent.SetRenderCustomDepth` (`self.StaticMesh`) false)
  (`SceneComponent.SetVisibility` (`self.Widget`) false false))

(fn `Laser Bounce`
  (params (`Hit?` :type Boolean) (`Laser Ref` :type "/Game/Personal/Blueprint_Mattia/BP_Switches/Lasers/BP_Laser Object Reference") (`Hit Result` :type "HitResult Structure"))
  (returns (`Spawn New Laser?` :type "/Game/Personal/Blueprint_Mattia/BP_Switches/Lasers/BP_Laser Object Reference"))
  (bind _laser_ref (`local.Laser Ref`))
  (bind _arrow (`self.Arrow`))
  (`self.LaserSpawn`
    (:`then`
      (if (not (`local.Hit?`))
        (`self.K2_DestroyActor` (`self.LaserSpawn`))))
    (:`else`
      (add `self.OnDestroyed` `Laser Ref` (`|CreateDelegate` :!event `OnDead`))
      (bind _returnvalue (`|SpawnActorFromClass` "/Game/Personal/Blueprint_Mattia/BP_Switches/Lasers/BP_Laser.BP_Laser_C" (`KismetMathLibrary.MakeTransform` (`SceneComponent.K2_GetComponentLocation` _arrow) (`KismetMathLibrary.MakeRotFromZ` (`SceneComponent.GetForwardVector` _arrow))) "Undefined" "MultiplyWithRoot" null (`/Game/Personal/Blueprint_Mattia/BP_Switches/Lasers/BP_LaserParent.LaserColor` _laser_ref) (`/Game/Personal/Blueprint_Mattia/BP_Switches/Lasers/BP_LaserParent.SpawnReference` _laser_ref) null))
      (set `self.LaserSpawn` _returnvalue)
      (`self.K2_AttachToComponent` _returnvalue (`self.Arrow`) "None" "KeepWorld" "KeepWorld" "KeepWorld" false))))

(fn `UserConstructionScript`
  (`parent.UserConstructionScript`))