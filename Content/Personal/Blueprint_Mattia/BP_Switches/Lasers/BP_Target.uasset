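; BP_Target is a laser puzzle target that lights up in the color of the laser hitting it.
; Laser Bounce stores the hit state in Active and passes it, with the laser's color, to PuzzleSolved.
; PuzzleSolved creates a new M_Solid dynamic material on SMParent at each call, setting Base Color to the laser color when hit or black otherwise.
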(fn `Laser Bounce`
  (params (`Hit?` :type Boolean) (`Laser Ref` :type "/Game/Personal/Blueprint_Mattia/BP_Switches/Lasers/BP_Laser Object Reference") (`Hit Result` :type "HitResult Structure"))
  (returns (`Spawn New Laser?` :type "/Game/Personal/Blueprint_Mattia/BP_Switches/Lasers/BP_Laser Object Reference"))
  (bind _output_get (set `self.Active` `Hit?`))
  (`self.PuzzleSolved` (`/Game/Personal/Blueprint_Mattia/BP_Switches/Lasers/BP_LaserParent.LaserColor` `Laser Ref`) _output_get)
  (return null))

(fn `PuzzleSolved`
  (params (`Color Laser` :type "LinearColor Structure") (bPickA :type Boolean))
  (bind _returnvalue (`PrimitiveComponent.CreateDynamicMaterialInstance` (`self.SM_Parent`) 0 "/Game/LevelPrototyping/Materials/M_Solid.M_Solid" "None"))
  (`MaterialInstanceDynamic.SetVectorParameterValue` _returnvalue "Base Color" (`KismetMathLibrary.SelectColor` `Color Laser` (struct) bPickA)))

(fn `UserConstructionScript`
  (`parent.UserConstructionScript`))