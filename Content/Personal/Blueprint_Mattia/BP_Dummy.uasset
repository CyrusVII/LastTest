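; BP_Dummy is a character dummy that goes limp as a physics body when its mesh is hit.
; The hit event sets a Done flag, turns on mesh physics simulation and collision, and disables capsule collision.
; A disconnected branch would move it toward the player with AIMoveTo until Done is set, then stop movement, but nothing triggers it.
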(event `self.Mesh.OnComponentHit`
  (params (HitComponent :type "PrimitiveComponent Object Reference") (OtherActor :type "Actor Object Reference") (OtherComp :type "PrimitiveComponent Object Reference") (NormalImpulse :type "Vector Structure") (Hit :type "HitResult Structure (by ref)"))
  (bind _mesh (`self.Mesh`))
  (set `self.Done` true)
  (`PrimitiveComponent.SetSimulatePhysics` _mesh true)
  (`PrimitiveComponent.SetCollisionEnabled` _mesh "QueryAndPhysics")
  (`PrimitiveComponent.SetCollisionEnabled` (`self.CapsuleComponent`) "NoCollision"))

(fn `UserConstructionScript`)