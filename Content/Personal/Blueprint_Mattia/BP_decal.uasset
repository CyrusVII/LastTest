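; BP_decal is a configurable decal actor with per-instance material, color tint, opacity and roughness.
; Its construction script applies DecalMaterial to the Decal component, then replaces it with a dynamic material instance created from it.
; It writes the Color Tint, Opacity and Roughtness parameters (the last spelled that way) from the actor's variables.
; The event graph holds only disabled default events, so all setup happens at construction.
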(fn `UserConstructionScript`
  (bind _decal (`self.Decal`))
  (`DecalComponent.SetDecalMaterial` _decal (`self.Decal Material`))
  (bind _returnvalue (`KismetMaterialLibrary.CreateDynamicMaterialInstance` (`DecalComponent.GetDecalMaterial` _decal)))
  (`DecalComponent.SetDecalMaterial` (`self.Decal`) _returnvalue)
  (`MaterialInstanceDynamic.SetVectorParameterValue` _returnvalue "Color Tint" (`self.Color Tint`))
  (`MaterialInstanceDynamic.SetScalarParameterValue` _returnvalue "Opacity" (`self.Opacity`))
  (`MaterialInstanceDynamic.SetScalarParameterValue` _returnvalue "Roughtness" (`self.Roughness`)))