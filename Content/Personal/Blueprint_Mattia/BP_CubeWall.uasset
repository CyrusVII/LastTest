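; BP_CubeWall is a colour-coded barrier that catches physics cubes of its matching value, or any cube as a Cube Destroyer.
; The construction script sets the wall material from CubeValue.
; On overlap with a cube's sphere, it freezes the cube, makes the player drop any held object and calls TooltipAction on the cube's button.
; A self-repeating half-second poll hides and disables the wall when locking is enabled and enough tagged Master_Template actors are active.
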(event `self.ReceiveBeginPlay`
  (bind _asbp_first_person_character (cast `/Game/Personal/Blueprint_Mattia/BP_FirstPersonCharacter` (`GameplayStatics.GetPlayerCharacter` 0)))
  (set `self.As BP First Person Character` _asbp_first_person_character)
  (`self.Tick`))

(event `Tick`
  (`|ExecutionSequence`
    (:`then_0`
      (bind _all_true (`self.TagTemplate`))
      (if _all_true
        (`self.SetActorHiddenInGame` true)
        (`PrimitiveComponent.SetCollisionEnabled` (`self.Box`) "NoCollision")
        (else
          (`self.SetActorHiddenInGame` false)
          (`PrimitiveComponent.SetCollisionEnabled` (`self.Box`) "QueryOnly"))))
    (:`then_1`
      (`KismetSystemLibrary.Delay` 0.5)
      (`self.Tick`))))

(event `self.Box.OnComponentBeginOverlap`
  (params (OverlappedComponent :type "PrimitiveComponent Object Reference") (OtherActor :type "Actor Object Reference") (OtherComp :type "PrimitiveComponent Object Reference") (OtherBodyIndex :type Integer) (bFromSweep :type Boolean) (SweepResult :type "HitResult Structure (by ref)"))
  (bind _staticmesh (`/Game/Personal/Blueprint_Mattia/BP_Switches/BP_Master_Template.StaticMesh` (`self.As BP Physic Cube`)))
  (bind _asbp_physic_cube (cast `/Game/Personal/Blueprint_Mattia/BP_Switches/BP_PhysicCube` OtherActor))
  (if (== OtherComp (`/Game/Personal/Blueprint_Mattia/BP_Switches/BP_PhysicCube.Sphere` _asbp_physic_cube))
    (bind _output_get (set `self.As BP Physic Cube` _asbp_physic_cube))
    (bind _button_ref (`/Game/Personal/Blueprint_Mattia/BP_Switches/BP_PhysicCube.Button Ref` _output_get)
      (:`then`
        (if (or (`|EnumEquality` (`self.CubeValue`) "NewEnumerator4") (`|EnumEquality` (`self.CubeValue`) (`/Game/Personal/Blueprint_Mattia/BP_Switches/BP_PhysicCube.ValueCube` _asbp_physic_cube)))
          (`/Engine/EditorBlueprintResources/StandardMacros.DoOnce` false :!label _label
            (:`Completed`
              (`PrimitiveComponent.SetEnableGravity` _staticmesh false)
              (`PrimitiveComponent.SetSimulatePhysics` _staticmesh false)
              (if (`/Game/Personal/Blueprint_Mattia/BP_FirstPersonCharacter.IsGrabbingObject` (`self.As BP First Person Character`))
                (`/Game/Personal/Blueprint_Mattia/BP_FirstPersonCharacter.Drop` (`self.As BP First Person Character`)))
              (`/Game/Personal/Blueprint_Mattia/BP_Switches/BP_Master_Template.Tooltip Action` _button_ref)
              (goto _label :!via `Reset`)))))
      (:`else`))))

(fn `TagTemplate`
  (returns (`All True` :type Boolean))
  (locals (`Locks Open` :type Integer))
  (if (`self.LockYesNo`)
    (bind _outactors (`GameplayStatics.GetAllActorsWithTag` (`self.Tag`)))
    (for _array_element _outactors
      (bind _asbp_master_template (cast `/Game/Personal/Blueprint_Mattia/BP_Switches/BP_Master_Template` _array_element))
      (if (`/Game/Personal/Blueprint_Mattia/BP_Switches/BP_Master_Template.Active` _asbp_master_template)
        (`/Engine/EditorBlueprintResources/StandardMacros.IncrementInt` (`local.Locks Open`))))
    (return (== (`local.Locks Open`) (`self.Locks`)))))

(fn `UserConstructionScript`
  (bind _wall (`self.Wall`))
  (bind _wall_2 (`self.Wall`))
  (switch `/Game/Personal/Blueprint_Mattia/Enum/E_ColorValue` (`self.CubeValue`)
    (:`NewEnumerator0`
      (`PrimitiveComponent.SetMaterial` _wall_2 0 "/Game/Personal/Blueprint_Mattia/Mesh/Material/MT_WallCube.MT_WallCube")
      (set `self.NoCubeOnOff` false))
    (:`NewEnumerator1`
      (`PrimitiveComponent.SetMaterial` _wall_2 0 "/Game/Personal/Blueprint_Mattia/Mesh/Material/MI_RedWallCube.MI_RedWallCube")
      (set `self.NoCubeOnOff` false))
    (:`NewEnumerator2`
      (`PrimitiveComponent.SetMaterial` _wall 0 "/Game/Personal/Blueprint_Mattia/Mesh/Material/MI_YellowWallCube.MI_YellowWallCube")
      (set `self.NoCubeOnOff` false))
    (:`NewEnumerator3`
      (`PrimitiveComponent.SetMaterial` _wall 0 "/Game/Personal/Blueprint_Mattia/Mesh/Material/MTI_WallCube_Neutre.MTI_WallCube_Neutre")
      (set `self.NoCubeOnOff` false))
    (:`NewEnumerator4`
      (`PrimitiveComponent.SetMaterial` _wall 0 "/Game/Personal/Blueprint_Mattia/Mesh/Material/MT_NoCube.MT_NoCube")
      (set `self.NoCubeOnOff` true))))